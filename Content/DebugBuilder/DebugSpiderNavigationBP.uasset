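; Debug Blueprint for the custom Spider navigation grid, driven by keyboard shortcuts.
; On BeginPlay it stores the first SpiderNavGridBuilder in the level and prints the key hints.
; R rebuilds the grid through the builder and then loads it, while Q draws the debug node connections.
; H reloads the grid and logs the result and node count without showing them on screen.
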(event `self.ReceiveBeginPlay`
  (`|ExecutionSequence`
    (:`then_0`
      (bind _outactors (`GameplayStatics.GetAllActorsOfClass` "/Script/SpiderNavigation.SpiderNavGridBuilder"))
      (if (> (`KismetArrayLibrary.Array_Length` _outactors) 0)
        (set `self.SpiderNavGridBuilder` (`KismetArrayLibrary.Array_Get` _outactors))
        (`KismetSystemLibrary.PrintString` "R - rebuild, Q - show connections" true true (struct :`G` 0.66 :`B` 1.0 :`A` 1.0) 20.0)))))

(event `Key|R`
  (params (Key :type "Key Structure" :default "AnyKey"))
  (:`Pressed`
    (`SpiderNavGridBuilder.BuildGrid` (`self.SpiderNavGridBuilder`))
    (`KismetSystemLibrary.PrintString` "Custom Nav Grid has been built")
    (`self.LoadGrid`)))

(event `Key|H`
  (params (Key :type "Key Structure" :default "AnyKey"))
  (:`Pressed`
    (bind _returnvalue (`self.LoadGrid`))
    (bind _returnvalue_2 (`self.GetNavNodesCount`))
    (`KismetSystemLibrary.PrintString` (`KismetStringLibrary.Concat_StrStr` "Custom Nav Grid Load Result: " (`KismetStringLibrary.Conv_BoolToString` _returnvalue) " Loaded: " (`KismetStringLibrary.Conv_IntToString` _returnvalue_2)) false)))

(event `Key|Q`
  (params (Key :type "Key Structure" :default "AnyKey"))
  (:`Pressed`
    (`self.DrawDebugRelations`)))

(fn `UserConstructionScript`)